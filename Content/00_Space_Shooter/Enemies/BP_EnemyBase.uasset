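; Base enemy actor for the space shooter that flies along its initial forward vector and fires on a timer.
; Tick moves it and, while firing is enabled, spawns ammo at FirePoint, either singly or as delayed three-shot bursts.
; Overlapping the player damages them, explodes and destroys the enemy.
; That collision and player ammo hits both roll a chance to spawn a power-up orb; ammo hits don't destroy it here.
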(event Custom|Fire
  (if (Variables|Default|GetBurst)
    (Game|SpawnActorfromClass (Variables|Default|GetAmmoType) (Transformation|GetWorldTransform (Variables|Default|GetFirePoint)) "Undefined" "MultiplyWithRoot" 0 0)
    (Utilities|FlowControl|Delay 0.4)
    (Game|SpawnActorfromClass (Variables|Default|GetAmmoType) (Transformation|GetWorldTransform (Variables|Default|GetFirePoint)) "Undefined" "MultiplyWithRoot" 0 0)
    (Utilities|FlowControl|Delay 0.4)
    (Game|SpawnActorfromClass (Variables|Default|GetAmmoType) (Transformation|GetWorldTransform (Variables|Default|GetFirePoint)) "Undefined" "MultiplyWithRoot" 0 0)
    (else
      (Game|SpawnActorfromClass (Variables|Default|GetAmmoType) (Transformation|GetWorldTransform (Variables|Default|GetFirePoint)) "Undefined" "MultiplyWithRoot" 0 0))))

(event Custom|Spawn%20Orb
  (if (<= (Math|Random|RandomFloatinRange 0.0 1.0) (Variables|Default|GetSpawn%20orb%20probability))
    (Game|SpawnActorfromClass (Variables|Default|GetPower%20Up%20Type) (Transformation|GetActorTransform) "Undefined" "MultiplyWithRoot" 0 0)))

(event EventBeginPlay
  (Variables|Default|SetMovementVector (Transformation|GetActorForwardVector)))

(event Collision|EventActorBeginOverlap
  (params (OtherActor :type Actor%20Object%20Reference))
  (bind _asss_player_character (Utilities|Casting|CastToSS_Player_Character OtherActor)
    (:then
      (Default|Damage _asss_player_character)
      (Effects|SpawnEmitteratLocation "/Game/StarterContent/Particles/P_Explosion.P_Explosion" (Transformation|GetActorLocation))
      (Audio|PlaySound2D "/Game/StarterContent/Audio/Explosion01.Explosion01" 1.0 1.0 0.0 0 0)
      (Utilities|FlowControl|Delay 0.1)
      (Actor|DestroyActor)
      (CallFunction|SpawnOrb))
    (:CastFailed
      (Utilities|Casting|CastToActor_Player_Ammo OtherActor)
      (CallFunction|SpawnOrb))))

(event EventTick
  (params (DeltaSeconds :type Float%20%28single-precision%29))
  ;[1 1 1] Comment
  (Transformation|SetActorLocation (+ (Transformation|GetActorLocation) (* (* DeltaSeconds (Variables|Default|GetSpeed)) (Variables|Default|GetMovementVector))) false false)
  (Variables|Default|SetShootCurrentTime (+ (Variables|Default|GetShootCurrentTime) DeltaSeconds))
  (if (> (Variables|Default|GetShootCurrentTime) (Variables|Default|GetDelayShoot))
    (if (Variables|Default|GetisFiring)
      (CallFunction|Fire)
      (Variables|Default|SetShootCurrentTime 0.0))))

(fn ConstructionScript)