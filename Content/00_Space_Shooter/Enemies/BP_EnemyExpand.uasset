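; BP_EnemyExpand is a space shooter enemy variant that grows wider the longer it exists.
; On BeginPlay it runs the parent logic, then sets a fixed speed and turns off firing and orb spawning.
; Each tick accumulates elapsed time to scale the actor linearly on X and Y, with Z fixed.
; It also resizes the Sphere collision radius from the length of that scale vector.
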(event EventBeginPlay
  (|CallParentFunction)
  (Variables|Default|SetSpeed 1e+02)
  (Variables|Default|SetCan%20Spawn%20orb false)
  (Variables|Default|SetisFiring false))

(event Collision|EventActorBeginOverlap
  (params (OtherActor :type Actor%20Object%20Reference))
  (|CallParentFunction OtherActor) ; This node is disabled and will not be called.\nDrag off pins to build functionality.
)

(event EventTick
  (params (DeltaSeconds :type Float%20%28single-precision%29))
  (|CallParentFunction DeltaSeconds)
  (bind _output_get (Variables|Default|SetCurrent%20mult (+ (Variables|Default|GetCurrent%20mult) DeltaSeconds)))
  (Transformation|SetActorScale3D (Math|Vector|MakeVector (* (Variables|Default|GetMultiply%20size%20factor) _output_get) (* (Variables|Default|GetMultiply%20size%20factor) _output_get) 1.0))
  (Components|Sphere|SetSphereRadius (Variables|Default|GetSphere) (* (Math|Vector|VectorLength (Math|Vector|MakeVector (* (Variables|Default|GetMultiply%20size%20factor) _output_get) (* (Variables|Default|GetMultiply%20size%20factor) _output_get) 1.0)) 45.0) true))

(fn ConstructionScript
  (|CallParentFunction))